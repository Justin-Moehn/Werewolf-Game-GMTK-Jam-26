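; BP_Key is a usable pickup item that unlocks locked buildings in front of the player.
; On use, it clears CanUseItem, then sphere-traces world objects a short distance along the player's look direction, with debug drawing enabled.
; The first locked BP_BuildingParent hit is unlocked, and the player destroys the held item, so a key is consumed only on a successful unlock.
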(event EventBeginPlay
  (|CallParentFunction) ; This node is disabled and will not be called.\nDrag off pins to build functionality.
)

(event EventTick
  (params (DeltaSeconds :type Float%20%28single-precision%29))
  (|CallParentFunction DeltaSeconds) ; This node is disabled and will not be called.\nDrag off pins to build functionality.
)

(event EventUseItem
  (bind _returnvalue (Game|GetPlayerCharacter 0))
  (bind _returnvalue_2 (Transformation|GetActorLocation _returnvalue))
  (|CallParentFunction)
  (if (Variables|Default|GetCanUseItem)
    (Variables|Default|SetCanUseItem false)
    (bind _asbp_player (Utilities|Casting|CastToBP_Player _returnvalue))
    (bind (_outhits _returnvalue_3) (Collision|MultiSphereTraceForObjects _returnvalue_2 (+ _returnvalue_2 (* (Math|Vector|GetForwardVector (Variables|/Game/Player/BP_Player.BP_Player_C|GetLookDirection _asbp_player)) 2e+02)) 75.0 (Utilities|Array|MakeArray "ObjectTypeQuery2" "ObjectTypeQuery1") false (Utilities|Array|MakeArray (Components|GetOwner)) "ForDuration"))
    (if _returnvalue_3
      (bind _array_element (Utilities|Array|ForEachLoopwithBreak _outhits :!label _label)
        (:LoopBody
          (bind _asbp_building_parent (Utilities|Casting|CastToBP_BuildingParent (.HitActor (Collision|BreakHitResult _array_element))))
          (if (Variables|/Game/Buildings/BP_BuildingParent.BP_BuildingParent_C|GetIsLocked _asbp_building_parent)
            (Default|UnLock _asbp_building_parent)
            (bind _asbp_player_2 (Utilities|Casting|CastToBP_Player (Game|GetPlayerCharacter 0)))
            (Default|DestroyItem _asbp_player_2)
            (goto _label Break)))))))