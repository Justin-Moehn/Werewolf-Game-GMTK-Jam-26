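; BP_ItemParent is a parent item Blueprint with drop and use events, judging by its name a base for pickup items.
; DropItem spawns the WorldPickupClass actor at the owner's location.
; UseItem, gated by CanUseItem, only prints a message and starts a cooldown timer that sets the flag true on expiry.
; Nothing here clears CanUseItem, so the cooldown does not block repeated use by itself.
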(event Custom|DropItem
  (Game|SpawnActorfromClass (Variables|Default|GetWorldPickupClass) (Math|Transform|MakeTransform (Transformation|GetActorLocation (Components|GetOwner)) "0, 0, 0" "1.000000,1.000000,1.000000") "Undefined" "MultiplyWithRoot" 0 0))

(event Custom|UseItem
  (if (Variables|Default|GetCanUseItem)
    (Development|PrintString "UsedItem")
    (Utilities|Time|SetTimerbyEvent (delegate Custom|CooldownOver) (Variables|Default|GetColldown))))

(event Custom|CooldownOver
  (Variables|Default|SetCanUseItem true))

(event EventBeginPlay)

(event EventTick
  (params (DeltaSeconds :type Float%20%28single-precision%29)))