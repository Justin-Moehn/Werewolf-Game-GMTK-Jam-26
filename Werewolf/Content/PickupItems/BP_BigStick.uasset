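; BP_BigStick is a usable pickup item that lets the player whack townsfolk and knock them back.
; On use, it clears CanUseItem and sphere-traces for pawns a short way along the player's LookDirection, with debug drawing on.
; The loop calls HitWithStick on the first hit, if it is a BP_TownsfolkParent, and launches it forward and slightly upward with a velocity-change impulse.
; This graph never re-enables CanUseItem.
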(event EventBeginPlay
  (|CallParentFunction))

(event EventTick
  (params (DeltaSeconds :type Float%20%28single-precision%29))
  (|CallParentFunction DeltaSeconds) ; This node is disabled and will not be called.\nDrag off pins to build functionality.
)

(event EventUseItem
  (bind _returnvalue (Game|GetPlayerCharacter 0))
  (bind _returnvalue_2 (Transformation|GetActorLocation _returnvalue))
  (|CallParentFunction)
  (if (Variables|Default|GetCanUseItem)
    (Variables|Default|SetCanUseItem false)
    (bind _asbp_player (Utilities|Casting|CastToBP_Player _returnvalue))
    (bind (_outhits _returnvalue_3) (Collision|MultiSphereTraceForObjects _returnvalue_2 (+ _returnvalue_2 (* (Math|Vector|GetForwardVector (Variables|/Game/Player/BP_Player.BP_Player_C|GetLookDirection _asbp_player)) 2e+02)) 75.0 (Utilities|Array|MakeArray "ObjectTypeQuery3") false (Utilities|Array|MakeArray (Components|GetOwner)) "ForDuration"))
    (if _returnvalue_3
      (bind _array_element (Utilities|Array|ForEachLoopwithBreak _outhits :!label _label)
        (:LoopBody
          (bind _asbp_townsfolk_parent (Utilities|Casting|CastToBP_TownsfolkParent (.HitActor (Collision|BreakHitResult _array_element))))
          (Default|HitwithStick _asbp_townsfolk_parent)
          (Physics|AddImpulse (Variables|/Script/Engine.Character|GetCharacterMovement _asbp_townsfolk_parent) (Math|Vector|MakeVector (.x (* (Math|Vector|GetForwardVector (Variables|/Game/Player/BP_Player.BP_Player_C|GetLookDirection _asbp_player)) 1e+03)) (.y (* (Math|Vector|GetForwardVector (Variables|/Game/Player/BP_Player.BP_Player_C|GetLookDirection _asbp_player)) 1e+03)) 1e+02) true)
          (goto _label Break))))))