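; Parent Blueprint for world item pickups, showing a name label on mouse hover and equipping an item on the player when interacted with or clicked.
; Interact runs once, only if the player has no item equipped, passing the item component class to the player before the pickup expires.
; Each hover restarts a short timer that hides the name widget once hovering stops, avoiding a separate hover-end event.
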(event Custom|StartNameTimer
  (Utilities|Time|ClearandInvalidateTimerbyHandle (Variables|Default|GetTimer))
  (bind _returnvalue (Utilities|Time|SetTimerbyEvent (delegate Custom|TimerFinished) 0.1))
  (Variables|Default|SetTimer _returnvalue))

(event Custom|TimerFinished
  (Rendering|SetVisibility (Variables|Default|GetWidget) false false))

(event EventBeginPlay
  (bind _aswb_townfolk_name (Utilities|Casting|CastToWB_TownfolkName (UserInterface|GetWidget (Variables|Default|GetWidget))))
  (Default|SetUpName _aswb_townfolk_name (Variables|Default|GetName) "" false 0.0))

(fn ConstructionScript)

(fn Interact
  (params (InteractedBy :type Actor%20Object%20Reference))
  (bind _asbp_player (Utilities|Casting|CastToBP_Player InteractedBy))
  (bind _itemequiped (Default|GetItemHeld _asbp_player))
  (if (not _itemequiped)
    (Utilities|FlowControl|DoOnce false
      (:Completed
        (Default|EquipItem _asbp_player (Variables|Default|GetItem%20Component%20Class))
        (Actor|SetLifeSpan 0.1)
        (return true)))))

(fn MouseClickon
  (bind _asbp_player (Utilities|Casting|CastToBP_Player (Game|GetPlayerCharacter 0)))
  (CallFunction|Interact _asbp_player)
  (return false))

(fn MouseHover
  (Rendering|SetVisibility (Variables|Default|GetWidget) true false)
  (CallFunction|StartNameTimer)
  (return true))