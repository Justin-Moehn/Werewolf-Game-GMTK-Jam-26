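; BP_MaleLover is a townsfolk character whose ability depends on whether its Lover shares a building with it.
; BeginPlay requests a random name before running parent logic, and SetWidget pushes name, title and points to the WB_TownfolkName widget.
; UseAbility searches the other building occupants for Lover and reports the ability as used only when the Lover is absent, naming itself as the user.
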(event Custom|SetWidget
  (bind _aswb_townfolk_name (Utilities|Casting|CastToWB_TownfolkName (UserInterface|GetWidget (Variables|Default|GetWidget))))
  (Default|SetUpName _aswb_townfolk_name (Variables|Default|GetName) (Variables|Default|GetTitle) true (Variables|Default|GetPoints)))

(event EventBeginPlay
  (CallFunction|GetRandomName true)
  (|CallParentFunction))

(event Collision|EventActorBeginOverlap
  (params (OtherActor :type Actor%20Object%20Reference)))

(event EventTick
  (params (DeltaSeconds :type Float%20%28single-precision%29)))

(fn ConstructionScript
  (|CallParentFunction))

(fn UseAbility
  (params (InIndex :type Integer) (OtherBuildingOcupents :type Array%20of%20BP%20Townsfolk%20Parent%20New%20Object%20References))
  (bind _array_element (Utilities|Array|ForEachLoopwithBreak OtherBuildingOcupents :!label _label)
    (:LoopBody
      (if (== _array_element (Variables|Default|GetLover))
        (LocalVariables|SetLCL_FoundLover true)
        (goto _label Break)))
    (:Completed
      (return (not (LocalVariables|GetLCL_FoundLover)) "NewEnumerator3" self 0))))