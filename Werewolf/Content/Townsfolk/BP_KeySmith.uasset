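; BP_KeySmith is a townsfolk actor, named as a key smith, that can drop a key pickup.
; On BeginPlay it gets a random name using a random boolean and sets points within a small range before running the parent BeginPlay.
; DropItem ignores its Item input and has a one-in-four chance to spawn BP_KeyPickUp at the actor's location.
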(event EventBeginPlay
  (CallFunction|GetRandomName (Math|Random|RandomBool))
  (CallFunction|SetPoints 2.0 6.0)
  (|CallParentFunction))

(event Collision|EventActorBeginOverlap
  (params (OtherActor :type Actor%20Object%20Reference)))

(event EventTick
  (params (DeltaSeconds :type Float%20%28single-precision%29)))

(fn ConstructionScript
  (|CallParentFunction))

(fn DropItem
  (params (Item :type BP%20World%20Pickup%20Parent%20Class%20Reference))
  (if (== (Math|Random|RandomIntegerinRange 1 4) 1)
    (Game|SpawnActorfromClass "/Game/PickupItems/WorldObjectPickups/BP_KeyPickUp.BP_KeyPickUp_C" (Math|Transform|MakeTransform (Transformation|GetActorLocation) "0, 0, 0" "1.000000,1.000000,1.000000") "Undefined" "MultiplyWithRoot" 0 0)))