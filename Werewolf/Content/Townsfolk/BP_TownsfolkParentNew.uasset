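; Base townsfolk NPC with a randomized name, gendered paper sprite and point value, which can follow the player or be put in a building.
; Following sets a blackboard state enum; a stick hit cancels it, and entering a building teleports the NPC far overhead in flying mode.
; Hover briefly shows a name tag, clicking opens an info widget, and dialogue appears for a timed, DoOnce-gated duration.
; UseAbility and DropItem are stubs.
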(event Custom|HitWithStick
  (Variables|Default|SetWasHit true)
  (CallFunction|SetFollowingPlayer false)
  (Utilities|Time|SetTimerbyEvent (delegate Custom|HitCooldownOver) 2.0))

(event Custom|HitCooldownOver
  (Variables|Default|SetWasHit false))

(event Custom|Setup)

(event Custom|HideNameAndTitle
  (Rendering|SetVisibility (Variables|Default|GetWidget) false false))

(event Custom|StartTitleCooldown
  (Utilities|Time|ClearandInvalidateTimerbyHandle (Variables|Default|GetTimer))
  (bind _returnvalue (Utilities|Time|SetTimerbyEvent (delegate Custom|HideNameAndTitle) 0.1))
  (Variables|Default|SetTimer _returnvalue))

(event Custom|UseDialogue
  (params (Dialogue :type String) (Time :type Float%20%28double-precision%29))
  (Utilities|FlowControl|DoOnce false
    (:Completed
      (Default|SetUpName (Variables|Default|GetDialogueWB) (Utilities|Text|ToText(String) Dialogue))
      (Rendering|SetVisibility (Variables|Default|GetDialogueWidgetr) true false)
      (Utilities|Time|SetTimerbyEvent (delegate Custom|StopDialogue) Time))))

(event Custom|StopDialogue
  (Rendering|SetVisibility (Variables|Default|GetDialogueWidgetr) false false)
  (Utilities|FlowControl|DoOnce false) ; enters at Reset
)

(event EventBeginPlay
  (bind _aswb_townfolk_name (Utilities|Casting|CastToWB_TownfolkName (UserInterface|GetWidget (Variables|Default|GetWidget))))
  (Default|SetUpName _aswb_townfolk_name (Variables|Default|GetName) (Variables|Default|GetTitle) true (Variables|Default|GetPoints))
  (Rendering|SetVisibility (Variables|Default|GetWidget) false false)
  (bind _aswb_townfolk_text (Utilities|Casting|CastToWB_TownfolkText (UserInterface|GetWidget (Variables|Default|GetDialogueWidgetr))))
  (Variables|Default|SetDialogueWB _aswb_townfolk_text))

(event EventMouseClickOff
  (Widget|RemovefromParent (Variables|Default|GetWidgetInfo))
  (Variables|Default|SetWidgetInfo 0)
  (Variables|Default|SetIsTalking false))

(fn ConstructionScript)

(fn SetFollowingPlayer
  (params (IsFollowing :type Boolean))
  (bind _returnvalue (Pawn|GetController))
  (bind _returnvalue_2 (Utilities|Name|MakeLiteralName "CurrentState"))
  (bind _returnvalue_3 (AI|GetBlackboard _returnvalue))
  (bind _output_get (Variables|Default|SetIsFollowingPlayer IsFollowing))
  (if _output_get
    (AI|Components|Blackboard|SetValueasEnum _returnvalue_3 _returnvalue_2 1)
    (else
      (AI|Components|Blackboard|SetValueasEnum _returnvalue_3 _returnvalue_2)
      (Components|Movement|StopMovementImmediately (Variables|Character|GetCharacterMovement)))))

(fn GetNearBuildings
  (return (Collision|GetOverlappingActors (Variables|Default|GetSphere) "/Game/Buildings/BP_BuildingParent.BP_BuildingParent_C" :!class /Script/Engine.PrimitiveComponent)))

(fn PutinBuilding
  (Transformation|SetActorLocation "0.000000,0.000000,100000.000000" false true)
  (CallFunction|SetFollowingPlayer false)
  (Pawn|Components|CharacterMovement|SetMovementMode (Variables|Character|GetCharacterMovement) "MOVE_Flying" 0))

(fn UseAbility
  (params (InIndex :type Integer) (OtherBuildingOcupents :type Array%20of%20BP%20Townsfolk%20Parent%20New%20Object%20References))
  (return false "NewEnumerator1" self InIndex))

(fn GetPointAMT
  (return (Variables|Default|GetPoints)))

(fn GetRandomName
  (params (IsMale :type Boolean))
  (if IsMale
    (bind _output_get (LocalVariables|SetFirstMaleName (Utilities|Enum|ByteToEnumE_FirstMaleName (Math|Conversions|ToByte(Integer) (Math|Random|RandomIntegerinRange 0 (- (|GetNumEnumEntries) 1))))))
    (LocalVariables|SetNewName (Utilities|String|EnumtoString _output_get))
    (else
      (bind _output_get_2 (LocalVariables|SetFirstFemaleName (Utilities|Enum|ByteToEnumE_FirstFemaleName (Math|Conversions|ToByte(Integer) (Math|Random|RandomIntegerinRange 0 (- (|GetNumEnumEntries) 1))))))
      (LocalVariables|SetNewName (Utilities|String|EnumtoString _output_get_2))))
  (bind _output_get_3 (LocalVariables|SetLastName (Utilities|Enum|ByteToEnumE_LastName (Math|Conversions|ToByte(Integer) (Math|Random|RandomIntegerinRange 0 (- (|GetNumEnumEntries) 1))))))
  (bind _output_get_4 (LocalVariables|SetNewName (Utilities|String|Append (LocalVariables|GetNewName) " " (Utilities|String|EnumtoString _output_get_3))))
  (Variables|Default|SetName (Utilities|Text|ToText(String) _output_get_4))
  (CallFunction|PickGender IsMale))

(fn SetPoints
  (params (Min :type Float%20%28double-precision%29) (Max :type Float%20%28double-precision%29))
  (Variables|Default|SetPoints (Math|Conversions|ToFloat(Integer) (Class|KismetMathLibrary|ToInt64(Float) (Math|Random|RandomFloatinRange Min Max)))))

(fn PickGender
  (params (Male? :type Boolean))
  (bind _papersprite (Variables|Default|GetPaperSprite))
  (if Male?
    (Rendering|Components|Sprite|SetSprite _papersprite (Variables|Default|GetMaleSprite))
    (else
      (Rendering|Components|Sprite|SetSprite _papersprite (Variables|Default|GetFemaleSprite)))))

(fn DropItem
  (params (Item :type BP%20World%20Pickup%20Parent%20Class%20Reference)))

(fn MouseClickon
  (Utilities|IsValid (Variables|Default|GetWidgetInfo)
    (:Is%20Not%20Valid
      (bind _returnvalue (UserInterface|CreateWidget (Variables|Default|GetInfoWidget)))
      (UserInterface|Viewport|AddtoViewport _returnvalue 0)
      (Variables|Default|SetWidgetInfo _returnvalue)
      (bind _aswb_townsfolk_wbparent (Utilities|Casting|CastToWB_TownsfolkWBParent _returnvalue))
      (Default|SetUpWidget _aswb_townsfolk_wbparent (>= (.x (Transformation|GetActorLocation (Game|GetPlayerCharacter 0))) (.x (Transformation|GetActorLocation))) (Variables|Default|GetName) (Variables|Default|GetTitle) (Variables|Default|GetDescription) (Variables|Default|GetIsFollowingPlayer) self)
      (Variables|Default|SetIsTalking true)
      (return true))))

(fn MouseHover
  (Rendering|SetVisibility (Variables|Default|GetWidget) true false)
  (CallFunction|StartTitleCooldown)
  (return true))