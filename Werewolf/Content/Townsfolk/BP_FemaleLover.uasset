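; BP_FemaleLover is a townsfolk character who pairs with BP_MaleLover and reacts to whether that partner shares her building.
; Shortly after getting a random name on BeginPlay, she scans all male lovers and cross-links with each unpaired one, keeping the last as Lover.
; Pairing gives both random love-themed descriptions naming the other and refreshes the male's widget.
; UseAbility reports the ability used only when her Lover is absent from the other occupants.
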(event Custom|SetLover
  (bind _name (Variables|Default|GetName))
  (bind _outactors (Actor|GetAllActorsOfClass "/Game/Townsfolk/BP_MaleLover.BP_MaleLover_C"))
  (for _array_element _outactors
    (Utilities|IsValid (Variables|/Game/Townsfolk/BP_MaleLover.BP_MaleLover_C|GetLover _array_element)
      (:Is%20Not%20Valid
        (Variables|Default|SetLover _array_element)
        (Variables|/Game/Townsfolk/BP_MaleLover.BP_MaleLover_C|SetLover _array_element self)
        (Variables|Default|SetDescription (.OutItem (Utilities|Array|Random (Utilities|Array|MakeArray (Utilities|Text|ToText(String) (Utilities|String|Append "“Where is " (Utilities|String|ToString(Text) (Variables|/Game/Townsfolk/BP_TownsfolkParentNew.BP_TownsfolkParentNew_C|GetName _array_element)) "?  
I need them!”")) (Utilities|Text|ToText(String) (Utilities|String|Append "\"I Love " (Utilities|String|ToString(Text) (Variables|/Game/Townsfolk/BP_TownsfolkParentNew.BP_TownsfolkParentNew_C|GetName _array_element)) ",  
I don't think I can live 
with out them. "))))))
        (Variables|/Game/Townsfolk/BP_TownsfolkParentNew.BP_TownsfolkParentNew_C|SetDescription _array_element (.OutItem (Utilities|Array|Random (Utilities|Array|MakeArray (Utilities|Text|ToText(String) (Utilities|String|Append "“Where is " (Utilities|String|ToString(Text) _name) "?  
I need them!”")) (Utilities|Text|ToText(String) (Utilities|String|Append "\"I Love " (Utilities|String|ToString(Text) _name) ",  
I don't think I can live 
with out them. "))))))
        (Default|SetWidget _array_element)))))

(event EventBeginPlay
  (CallFunction|GetRandomName false)
  (Utilities|FlowControl|Delay 0.2)
  (CallFunction|SetLover)
  (|CallParentFunction)
  (Utilities|FlowControl|Delay 5.0))

(event Collision|EventActorBeginOverlap
  (params (OtherActor :type Actor%20Object%20Reference)))

(event EventTick
  (params (DeltaSeconds :type Float%20%28single-precision%29)))

(fn ConstructionScript
  (|CallParentFunction))

(fn UseAbility
  (params (InIndex :type Integer) (OtherBuildingOcupents :type Array%20of%20BP%20Townsfolk%20Parent%20New%20Object%20References))
  (bind _array_element (Utilities|Array|ForEachLoopwithBreak OtherBuildingOcupents :!label _label)
    (:LoopBody
      (if (== _array_element (Variables|Default|GetLover))
        (LocalVariables|SetLCL_FoundLover true)
        (goto _label Break)))
    (:Completed
      (return (not (LocalVariables|GetLCL_FoundLover)) "NewEnumerator3" self 0))))