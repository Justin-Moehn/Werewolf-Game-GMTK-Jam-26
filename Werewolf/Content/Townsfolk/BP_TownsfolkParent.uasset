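; Parent Blueprint for townsfolk NPCs that can follow the player, be talked to and be put in buildings.
; Hovering reveals a name/title widget through a restarted short hide timer, while clicking opens an info widget aware of the player's side.
; Follow state drives a Blackboard enum, and stick hits cancel it with a brief cooldown.
; Stored townsfolk teleport far overhead in flying mode; Setup and UseAbility are empty hooks.
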(event Custom|HitWithStick
  (Variables|Default|SetWasHit true)
  (CallFunction|SetFollowingPlayer false)
  (Utilities|Time|SetTimerbyEvent (delegate Custom|HitCooldownOver) 2.0))

(event Custom|HitCooldownOver
  (Variables|Default|SetWasHit false))

(event Custom|Setup)

(event Custom|HideNameAndTitle
  (Rendering|SetVisibility (Variables|Default|GetWidget) false false))

(event Custom|StartTitleCooldown
  (Utilities|Time|ClearandInvalidateTimerbyHandle (Variables|Default|GetTimer))
  (bind _returnvalue (Utilities|Time|SetTimerbyEvent (delegate Custom|HideNameAndTitle) 0.1))
  (Variables|Default|SetTimer _returnvalue))

(event Custom|UseAbility)

(event EventBeginPlay
  (bind _aswb_townfolk_name (Utilities|Casting|CastToWB_TownfolkName (UserInterface|GetWidget (Variables|Default|GetWidget))))
  (Default|SetUpName _aswb_townfolk_name (Variables|Default|GetName) (Variables|Default|GetTitle))
  (Rendering|SetVisibility (Variables|Default|GetWidget) false false))

(event EventMouseClickOff
  (Widget|RemovefromParent (Variables|Default|GetWidgetInfo))
  (Variables|Default|SetWidgetInfo 0)
  (Variables|Default|SetIsTalking false))

(fn ConstructionScript)

(fn SetFollowingPlayer
  (params (IsFollowing :type Boolean))
  (bind _returnvalue (Pawn|GetController))
  (bind _returnvalue_2 (Utilities|Name|MakeLiteralName "CurrentState"))
  (bind _returnvalue_3 (AI|GetBlackboard _returnvalue))
  (bind _output_get (Variables|Default|SetIsFollowingPlayer IsFollowing))
  (if _output_get
    (AI|Components|Blackboard|SetValueasEnum _returnvalue_3 _returnvalue_2 1)
    (else
      (AI|Components|Blackboard|SetValueasEnum _returnvalue_3 _returnvalue_2)
      (Components|Movement|StopMovementImmediately (Variables|Character|GetCharacterMovement)))))

(fn GetNearBuildings
  (return (Collision|GetOverlappingActors (Variables|Default|GetSphere) "/Game/Buildings/BP_BuildingParent.BP_BuildingParent_C" :!class /Script/Engine.PrimitiveComponent)))

(fn PutinBuilding
  (Transformation|SetActorLocation "0.000000,0.000000,100000.000000" false true)
  (CallFunction|SetFollowingPlayer false)
  (Pawn|Components|CharacterMovement|SetMovementMode (Variables|Character|GetCharacterMovement) "MOVE_Flying" 0))

(fn MouseClickon
  (Utilities|IsValid (Variables|Default|GetWidgetInfo)
    (:Is%20Not%20Valid
      (bind _returnvalue (UserInterface|CreateWidget (Variables|Default|GetInfoWidget)))
      (UserInterface|Viewport|AddtoViewport _returnvalue 0)
      (Variables|Default|SetWidgetInfo _returnvalue)
      (bind _aswb_townsfolk_wbparent (Utilities|Casting|CastToWB_TownsfolkWBParent _returnvalue))
      (Default|SetUpWidget _aswb_townsfolk_wbparent (>= (.x (Transformation|GetActorLocation (Game|GetPlayerCharacter 0))) (.x (Transformation|GetActorLocation))) (Variables|Default|GetName) (Variables|Default|GetTitle) (Variables|Default|GetDescription) (Variables|Default|GetIsFollowingPlayer) self)
      (Variables|Default|SetIsTalking true)
      (return true))))

(fn MouseHover
  (Rendering|SetVisibility (Variables|Default|GetWidget) true false)
  (CallFunction|StartTitleCooldown)
  (return true))