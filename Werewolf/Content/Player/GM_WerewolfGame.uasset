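; Werewolf game mode that ends a scoring round on a looping 15-second timer and shows the results in an end-of-round widget.
; CalculateScore gathers all townsfolk and buildings, marking unprotected townsfolk and those reported dead by each building as casualties.
; Survivors then use abilities, where a Heal moves one casualty back to the living, uses the Doctor's herb and logs a notification.
; Survivors' points form the round score, added to a running total.
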(event Custom|CustomEvent
  (bind (_livingtownsfolk _livingamt _deadamt _score) (CallFunction|CalculateScore))
  (Variables|Default|SetTotalScore (+ (Variables|Default|GetTotalScore) (Variables|Default|GetScore)))
  (bind _returnvalue (UserInterface|CreateWidget "/Game/Widgets/WB_EndRoundScore.WB_EndRoundScore_C" 0 (Math|Conversions|ToFloat(Integer) _livingamt) (Math|Conversions|ToFloat(Integer) _deadamt) _score (Variables|Default|GetTotalScore) (Variables|Default|GetUpdateSheetNotifications)))
  (UserInterface|Viewport|AddtoViewport _returnvalue 0))

(event EventBeginPlay
  (Utilities|Time|SetTimerbyEvent (delegate Custom|CustomEvent) 15.0 true))

(fn ConstructionScript)

(fn CalculateScore
  (bind _alldeadtownsfolk (Variables|Default|GetAllDeadTownsfolk))
  (bind _alldeadtownsfolk_2 (Variables|Default|GetAllDeadTownsfolk))
  (bind _returnvalue (Utilities|Array|Length _alldeadtownsfolk_2))
  (Utilities|Array|Clear (Variables|Default|GetUpdateSheetNotifications))
  (Variables|Default|SetScore 0.0)
  (Utilities|Array|Clear (Variables|Default|GetAllTownsfolk))
  (Utilities|Array|Clear (Variables|Default|GetAllBuildings))
  (Utilities|Array|Clear (Variables|Default|GetAllDeadTownsfolk))
  (bind _outactors (Actor|GetAllActorsOfClass "/Game/Townsfolk/BP_TownsfolkParent.BP_TownsfolkParent_C"))
  (Variables|Default|SetAllTownsfolk _outactors)
  (bind _outactors_2 (Actor|GetAllActorsOfClass "/Game/Buildings/BP_BuildingParent.BP_BuildingParent_C"))
  (Variables|Default|SetAllBuildings _outactors_2)
  (Variables|Default|SetTotalTownsfolkAMT (Utilities|Array|Length (Variables|Default|GetAllTownsfolk)))
  (for _array_element (Variables|Default|GetAllTownsfolk)
    (if (not (Variables|/Game/Townsfolk/BP_TownsfolkParent.BP_TownsfolkParent_C|GetIsProtected _array_element))
      (Utilities|Array|Add (Variables|Default|GetAllDeadTownsfolk) _array_element)))
  (for _array_element_2 (Variables|Default|GetAllBuildings)
    (bind _deadtownsfolk (Default|CalculateScoreinBuilding _array_element_2))
    (for _array_element_3 _deadtownsfolk
      (Utilities|Array|Add (Variables|Default|GetAllDeadTownsfolk) _array_element_3)))
  (bind _array_element_4 (Utilities|Array|ForEachLoopwithBreak (Variables|Default|GetAllDeadTownsfolk))
    (:LoopBody
      (if (Utilities|Array|ContainsItem (Variables|Default|GetAllTownsfolk) _array_element_4)
        (Utilities|Array|RemoveItem (Variables|Default|GetAllTownsfolk) _array_element_4)))
    (:Completed
      (for (_array_element_5 _array_index) (Variables|Default|GetAllTownsfolk)
        (bind (_usedability _abilityname _usedby) (Default|UseAbility _array_element_5 _array_index))
        (if _usedability
          (switch Utilities|FlowControl|Switch|SwitchonE_TownsfolkAbilities _abilityname
            (:NewEnumerator2
              (if (Utilities|Array|IsNotEmpty (Variables|Default|GetAllDeadTownsfolk))
                (if (< _returnvalue 1)
                  (LocalVariables|SetLCL_RandomInt (Math|Random|RandomIntegerinRange 0 (- _returnvalue 1)))
                  (else
                    (LocalVariables|SetLCL_RandomInt 0)))
                (bind _returnvalue_2 (Utilities|Array|Add (Variables|Default|GetAllTownsfolk) (Utilities|Array|Get(acopy) _alldeadtownsfolk (LocalVariables|GetLCL_RandomInt))))
                (Utilities|Array|RemoveIndex _alldeadtownsfolk (LocalVariables|GetLCL_RandomInt))
                (Utilities|Array|Add (Variables|Default|GetUpdateSheetNotifications) (Utilities|String|Append (Utilities|String|ToString(Text) (Variables|/Game/Townsfolk/BP_TownsfolkParent.BP_TownsfolkParent_C|GetName _usedby)) " has saved  
" (Utilities|String|ToString(Text) (Variables|/Game/Townsfolk/BP_TownsfolkParent.BP_TownsfolkParent_C|GetName (Utilities|Array|Get(acopy) (Variables|Default|GetAllTownsfolk) _returnvalue_2))) " from certain 
death."))
                (Development|PrintString "Hello")
                (bind _asbp_doctor (Utilities|Casting|CastToBP_Doctor _usedby))
                (Variables|/Game/Townsfolk/BP_Doctor.BP_Doctor_C|SetHasHerb _asbp_doctor false))))))
      (for _array_element_6 (Variables|Default|GetAllTownsfolk)
        (bind _score (Default|GetPointAMT _array_element_6))
        (Variables|Default|SetScore (+ _score (Variables|Default|GetScore))))
      (return (Variables|Default|GetAllTownsfolk) (Utilities|Array|Length (Variables|Default|GetAllTownsfolk)) (Utilities|Array|Length (Variables|Default|GetAllDeadTownsfolk)) (Variables|Default|GetScore)))))