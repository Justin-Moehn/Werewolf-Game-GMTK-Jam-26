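; Player character with camera-relative movement, HUD, pause menu and one held item.
; StartDay teleports it to the town hall spawn and enables movement, hovering and clicking, which EndDay disables.
; Per-tick cursor traces set HoverActor via interface messages; clicking nearby targets locks movement and hover until clicked again.
; Items are runtime-added BP_ItemParent components mirrored on the HUD; Interact and DropItem are not wired to input.
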(event Custom|Interact
  (bind _returnvalue (Transformation|GetActorLocation))
  (bind (_outhits _returnvalue_2) (Collision|MultiSphereTraceByChannel _returnvalue _returnvalue 2.5e+02 "TraceTypeQuery1" false 0 "ForDuration"))
  (if _returnvalue_2
    (bind _array_element (Utilities|Array|ForEachLoopwithBreak _outhits :!label _label)
      (:LoopBody
        (bind _interacted (Class|BPIIInteractable|Interact(Message) (.HitActor (Collision|BreakHitResult _array_element)) self))
        (if _interacted
          (goto _label Break))))))

(event Custom|GetHoverNames
  (bind _returnvalue (Game|GetPlayerController 0))
  (bind _hitresult (Game|Player|GetHitResultUnderCursorbyChannel _returnvalue "TraceTypeQuery2" true))
  (bind _hitactor (Collision|BreakHitResult _hitresult))
  (if (Variables|Default|GetCanGetHoverNames)
    (bind _onhover (Class|BPIIMouseSelectable|MouseHover(Message) _hitactor))
    (if _onhover
      (Variables|Default|SetHoverActor _hitactor)
      (else
        (Variables|Default|SetHoverActor 0)))))

(event Custom|DestroyItem
  (Utilities|IsValid (Variables|Default|GetItemComponent)
    (:Is%20Valid
      (bind _asbp_item_parent (Utilities|Casting|CastToBP_ItemParent (Variables|Default|GetItemComponent)))
      (Default|DestroyItem _asbp_item_parent)
      (Variables|Default|SetItemComponent 0)
      (Default|UnequipItem (Variables|Default|GetHud)))))

(event Custom|EndDay
  (Variables|Default|SetCanMove false)
  (Variables|Default|SetCanGetHoverNames false)
  (Variables|Default|SetCanClick false))

(event Custom|StartDay
  (Variables|Default|SetCanMove true)
  (Variables|Default|SetCanGetHoverNames true)
  (Variables|Default|SetCanClick true)
  (bind _returnvalue (Actor|GetActorOfClass "/Game/Buildings/BP_TownHall.BP_TownHall_C"))
  (Transformation|SetWorldLocation (Variables|Default|GetCapsuleComponent) (Transformation|GetWorldLocation (Variables|/Game/Buildings/BP_BuildingParent.BP_BuildingParent_C|GetSpawnLocation _returnvalue)) false true))

(event Input|EnhancedActionEvents|EnhancedInputActionIA_Move
  (params (ActionValue :type Vector%202D%20Structure) (ElapsedSeconds :type Float%20%28double-precision%29) (TriggeredSeconds :type Float%20%28double-precision%29) (InputAction :type Input%20Action%20Object%20Reference :default "/Game/Input/InputActions/IA_Move.IA_Move"))
  (bind (_x _y) (Math|Vector2D|BreakVector2D ActionValue))
  ;[0.15 0.15 0.15 0.5] Player movement
  (:Triggered
    (if (Variables|Default|GetCanMove)
      (CallFunction|Move _x _y)))
  (:Started
    (if (Variables|Default|GetCanMove)
      (Variables|Default|SetIsMoving true)))
  (:Canceled
    (Variables|Default|SetIsMoving false :!label _label))
  (:Completed
    (goto _label)))

(event Input|EnhancedActionEvents|EnhancedInputActionIA_Interact
  (params (ActionValue :type Boolean) (ElapsedSeconds :type Float%20%28double-precision%29) (TriggeredSeconds :type Float%20%28double-precision%29) (InputAction :type Input%20Action%20Object%20Reference :default "/Game/Input/InputActions/IA_Interact.IA_Interact")))

(event Input|EnhancedActionEvents|EnhancedInputActionIA_DropItem
  (params (ActionValue :type Boolean) (ElapsedSeconds :type Float%20%28double-precision%29) (TriggeredSeconds :type Float%20%28double-precision%29) (InputAction :type Input%20Action%20Object%20Reference :default "/Game/Input/InputActions/IA_DropItem.IA_DropItem")))

(event Input|EnhancedActionEvents|EnhancedInputActionIA_UseItem
  (params (ActionValue :type Boolean) (ElapsedSeconds :type Float%20%28double-precision%29) (TriggeredSeconds :type Float%20%28double-precision%29) (InputAction :type Input%20Action%20Object%20Reference :default "/Game/Input/InputActions/IA_UseItem.IA_UseItem"))
  (bind _itemcomponent (Variables|Default|GetItemComponent))
  (:Started
    (Utilities|IsValid _itemcomponent
      (:Is%20Valid
        (bind _asbp_item_parent (Utilities|Casting|CastToBP_ItemParent _itemcomponent))
        (Default|UseItem _asbp_item_parent)))))

(event Input|EnhancedActionEvents|EnhancedInputActionIA_SelectMember
  (params (ActionValue :type Boolean) (ElapsedSeconds :type Float%20%28double-precision%29) (TriggeredSeconds :type Float%20%28double-precision%29) (InputAction :type Input%20Action%20Object%20Reference :default "/Game/Input/InputActions/IA_SelectMember.IA_SelectMember"))
  (bind _hoveractor (Variables|Default|GetHoverActor))
  (bind _hoveractor_2 (Variables|Default|GetHoverActor))
  (:Started
    (if (Variables|Default|GetCanClick)
      (if (Variables|Default|GetCanGetHoverNames)
        (Utilities|IsValid _hoveractor_2
          (:Is%20Valid
            (if (< (Math|Vector|Distance(Vector) (Transformation|GetActorLocation _hoveractor_2) (Transformation|GetActorLocation)) 4.5e+02)
              (bind _stopmovement (Class|BPIIMouseSelectable|MouseClickon(Message) _hoveractor_2 (Variables|Default|GetHoldingShift)))
              (if _stopmovement
                (Variables|Default|SetCanMove false)
                (Variables|Default|SetCanGetHoverNames false)))))
        (else
          (Utilities|IsValid _hoveractor
            (:Is%20Valid
              (Class|BPIIMouseSelectable|MouseClickOff(Message) _hoveractor)
              (Variables|Default|SetCanGetHoverNames true)
              (Variables|Default|SetCanMove true))))))))

(event EventBeginPlay
  (bind _returnvalue (Game|GetPlayerController 0))
  ;[0.15 0.15 0.15 0.5] Set up hud and ui
  (bind _returnvalue_2 (UserInterface|CreateWidget "/Game/Widgets/WB_PlayerHUD.WB_PlayerHUD_C"))
  (UserInterface|Viewport|AddtoViewport _returnvalue_2 0)
  (Variables|Default|SetHud _returnvalue_2)
  (Variables|/Script/Engine.PlayerController|SetbShowMouseCursor _returnvalue true)
  (Variables|/Script/Engine.PlayerController|SetbEnableMouseOverEvents _returnvalue true))

(event EventTick
  (params (DeltaSeconds :type Float%20%28single-precision%29))
  (CallFunction|GetHoverNames))

(event Input|KeyboardEvents|Divide
  (params (Key :type Key%20Structure :default "None"))
  (:Pressed
    (bind _outactors (Actor|GetAllActorsOfClass "/Game/Buildings/BP_TownHall.BP_TownHall_C"))
    (for _array_element _outactors
      (Default|EnmptyHouse _array_element))))

(event Input|KeyboardEvents|Escape
  (params (Key :type Key%20Structure :default "None"))
  (:Pressed
    (bind _returnvalue (UserInterface|CreateWidget "/Game/Widgets/WB_Pause.WB_Pause_C"))
    (UserInterface|Viewport|AddtoViewport _returnvalue 0)))

(event Input|KeyboardEvents|P
  (params (Key :type Key%20Structure :default "None"))
  (:Pressed
    (bind _returnvalue (UserInterface|CreateWidget "/Game/Widgets/WB_Pause.WB_Pause_C"))
    (UserInterface|Viewport|AddtoViewport _returnvalue 0)))

(event Input|KeyboardEvents|LeftShift
  (params (Key :type Key%20Structure :default "None"))
  (:Pressed
    (Variables|Default|SetHoldingShift true))
  (:Released
    (Variables|Default|SetHoldingShift false)))

(fn ConstructionScript)

(fn Move
  (params (X :type Float%20%28double-precision%29) (Y :type Float%20%28double-precision%29))
  (bind _returnvalue (Transformation|GetActorLocation))
  (bind _returnvalue_2 (Pawn|GetControlRotation :!class /Script/Engine.Pawn))
  (if (> (Math|Float|Absolute(Float) (Math|Vector2D|Vector2DLength (Math|Vector2D|MakeVector2D X Y))) 0.2)
    (Pawn|Input|AddMovementInput (Math|Vector|GetRightVector (Math|Rotator|MakeRotator (.roll _returnvalue_2) 0.0 (.yaw _returnvalue_2))) X false)
    (Pawn|Input|AddMovementInput (Math|Vector|GetForwardVector (Math|Rotator|MakeRotator 0.0 0.0 (.yaw (Pawn|GetControlRotation :!class /Script/Engine.Pawn)))) Y false)
    (Transformation|SetWorldRotation (Variables|Default|GetLookDirection) (Math|Rotator|FindLookatRotation _returnvalue (+ _returnvalue (* (Pawn|Components|PawnMovement|GetLastInputVector (Variables|Character|GetCharacterMovement)) 5e+01))) false false)))

(fn GetItemHeld
  (bind _itemcomponent (Variables|Default|GetItemComponent))
  (return (Utilities|IsValid _itemcomponent) _itemcomponent))

(fn EquipItem
  (params (ItemClass :type Actor%20Component%20Class%20Reference))
  (bind _returnvalue (Game|AddComponentbyClass ItemClass))
  (bind _output_get (Variables|Default|SetItemComponent _returnvalue))
  (bind _asbp_item_parent (Utilities|Casting|CastToBP_ItemParent _output_get))
  (Default|EquipItem (Variables|Default|GetHud) (Variables|/Game/PickupItems/BP_ItemParent.BP_ItemParent_C|GetItemImage _asbp_item_parent)))

(fn DropItem
  (Utilities|IsValid (Variables|Default|GetItemComponent)
    (:Is%20Valid
      (bind _asbp_item_parent (Utilities|Casting|CastToBP_ItemParent (Variables|Default|GetItemComponent)))
      (Default|DropItem _asbp_item_parent)
      (Variables|Default|SetItemComponent 0)
      (Default|UnequipItem (Variables|Default|GetHud)))))