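; Town hall building, named as a tutorial variant, that opens an info widget when clicked.
; MouseClickOn creates the widget only if none is valid, then fills it with the name, description, remaining-capacity text and a reference to the building.
; An IsOnRight flag comes from comparing the player character's X position with the building's.
; The event graph and construction script add no logic of their own.
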(event EventBeginPlay
  (|CallParentFunction) ; This node is disabled and will not be called.\nDrag off pins to build functionality.
)

(event Collision|EventActorBeginOverlap
  (params (OtherActor :type Actor%20Object%20Reference)))

(event EventTick
  (params (DeltaSeconds :type Float%20%28single-precision%29)))

(fn ConstructionScript
  (|CallParentFunction))

(fn MouseClickon
  (Utilities|IsValid (Variables|Default|GetWidgetInfo)
    (:Is%20Not%20Valid
      (bind _returnvalue (UserInterface|CreateWidget (Variables|Default|GetInfoWidget)))
      (UserInterface|Viewport|AddtoViewport _returnvalue 0)
      (bind _output_get (Variables|Default|SetWidgetInfo _returnvalue))
      (bind _aswb_building_wbtown_hall (Utilities|Casting|CastToWB_BuildingWBTownHall _output_get))
      (Default|SetUpWidget _aswb_building_wbtown_hall (>= (.x (Transformation|GetActorLocation (Game|GetPlayerCharacter 0))) (.x (Transformation|GetActorLocation))) (Variables|Default|GetName) (Utilities|Text|ToText(String) (Utilities|String|Append (Utilities|String|ToString(Float) (Variables|Default|GetCapacity)) " out of " (Utilities|String|ToString(Float) (Variables|Default|GetMaxCapacity)) " spots left")) (Variables|Default|GetDescription) self)
      (return true))))