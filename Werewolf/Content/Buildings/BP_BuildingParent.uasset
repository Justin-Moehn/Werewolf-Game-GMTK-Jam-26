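; Base building for the werewolf game, where townsfolk shelter as protected occupants up to a size-based capacity.
; Locked or broken buildings refuse entry, and a world widget shows state or capacity on hover, hidden by a retriggered timer, while clicking opens an info panel.
; Scoring runs occupant abilities (Murder, Lost Lover), returning living and dead lists and queuing game mode notifications.
; Emptying ejects occupants at the spawn point and may randomly lock the building.
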(event Custom|StartHoverCooldown
  (Utilities|Time|ClearandInvalidateTimerbyHandle (Variables|Default|GetTimer))
  (bind _returnvalue (Utilities|Time|SetTimerbyEvent (delegate Custom|CooldownFinished) 0.1))
  (Variables|Default|SetTimer _returnvalue))

(event Custom|CooldownFinished
  (Rendering|SetVisibility (Variables|Default|GetWidget) false false))

(event Custom|UnLock
  (Variables|Default|SetIsLocked false)
  (bind _aswb_building_name (Utilities|Casting|CastToWB_BuildingName (UserInterface|GetWidget (Variables|Default|GetWidget))))
  (Default|SetUpName _aswb_building_name (Variables|Default|GetName) (Utilities|Text|ToText(String) (Utilities|String|Append (Utilities|String|ToString(Float) (Variables|Default|GetCapacity)) " out of " (Utilities|String|ToString(Float) (Variables|Default|GetMaxCapacity)) " spots left"))))

(event Custom|SetBroken
  (params (IsBroken :type Boolean))
  (bind _name (Variables|Default|GetName))
  (bind _output_get (Variables|Default|SetIsBroken IsBroken))
  (if _output_get
    (bind _aswb_building_name (Utilities|Casting|CastToWB_BuildingName (UserInterface|GetWidget (Variables|Default|GetWidget))))
    (Default|SetUpName _aswb_building_name (Variables|Default|GetName) "Broken: Requires Hammer")
    (else
      (bind _aswb_building_name_2 (Utilities|Casting|CastToWB_BuildingName (UserInterface|GetWidget (Variables|Default|GetWidget))))
      (if (Variables|Default|GetIsLocked)
        (Default|SetUpName _aswb_building_name_2 _name "Locked: Requires Key")
        (else
          (Default|SetUpName _aswb_building_name_2 _name (Utilities|Text|ToText(String) (Utilities|String|Append (Utilities|String|ToString(Float) (Variables|Default|GetCapacity)) " out of " (Utilities|String|ToString(Float) (Variables|Default|GetMaxCapacity)) " spots left"))))))))

(event EventBeginPlay
  (bind _name (Variables|Default|GetName))
  (bind _aswb_building_name (Utilities|Casting|CastToWB_BuildingName (UserInterface|GetWidget (Variables|Default|GetWidget))))
  (if (Variables|Default|GetIsLocked)
    (Default|SetUpName _aswb_building_name _name "Locked: Requires Key")
    (else
      (Default|SetUpName _aswb_building_name _name (Utilities|Text|ToText(String) (Utilities|String|Append (Utilities|String|ToString(Float) (Variables|Default|GetCapacity)) " out of " (Utilities|String|ToString(Float) (Variables|Default|GetMaxCapacity)) " spots left")))))
  (CallFunction|SetBroken (Variables|Default|GetIsBroken)))

(event EventTick
  (params (DeltaSeconds :type Float%20%28single-precision%29)))

(event EventMouseClickOff
  (Widget|RemovefromParent (Variables|Default|GetWidgetInfo))
  (Variables|Default|SetWidgetInfo 0))

(fn ConstructionScript)

(fn GetCapacity
  (return (Variables|Default|GetCapacity)))

(fn AddtoBuilding
  (params (NewTownsfolk :type BP%20Townsfolk%20Parent%20New%20Object%20Reference%20%28by%20ref%29))
  (bind _size (Variables|/Game/Townsfolk/BP_TownsfolkParentNew.BP_TownsfolkParentNew_C|GetSize NewTownsfolk))
  (if (Math|Boolean|ANDBoolean (<= (+ _size (Variables|Default|GetCapacity)) (Variables|Default|GetMaxCapacity)) (not (Variables|Default|GetIsLocked)) (not (Variables|Default|GetIsBroken)))
    (Variables|Default|SetCapacity (+ _size (Variables|Default|GetCapacity)))
    (Utilities|Array|Add (Variables|Default|GetTownsfolk) NewTownsfolk)
    (Default|PutinBuilding NewTownsfolk)
    (Variables|/Game/Townsfolk/BP_TownsfolkParentNew.BP_TownsfolkParentNew_C|SetIsProtected NewTownsfolk true)
    (bind _aswb_building_name (Utilities|Casting|CastToWB_BuildingName (UserInterface|GetWidget (Variables|Default|GetWidget))))
    (Default|SetUpName _aswb_building_name (Variables|Default|GetName) (Utilities|Text|ToText(String) (Utilities|String|Append (Utilities|String|ToString(Float) (Variables|Default|GetCapacity)) " out of " (Utilities|String|ToString(Float) (Variables|Default|GetMaxCapacity)) " spots left")))))

(fn RemovefromBuilding
  (params (Index :type Integer))
  (bind _townsfolk (Variables|Default|GetTownsfolk))
  (bind _spawnlocation (Variables|Default|GetSpawnLocation))
  (bind _returnvalue (Transformation|GetWorldLocation _spawnlocation))
  (bind _output (Utilities|Array|Get(acopy) _townsfolk Index))
  (Utilities|IsValid _output
    (:Is%20Valid
      (Variables|/Game/Townsfolk/BP_TownsfolkParentNew.BP_TownsfolkParentNew_C|SetIsTalking _output false)
      (AI|Components|Blackboard|SetValueasEnum (AI|GetBlackboard (Pawn|GetController _output)) (Utilities|Name|MakeLiteralName "CurrentState"))
      (Variables|Default|SetCapacity (- (Variables|Default|GetCapacity) (Variables|/Game/Townsfolk/BP_TownsfolkParentNew.BP_TownsfolkParentNew_C|GetSize _output)))
      (Variables|/Game/Townsfolk/BP_TownsfolkParentNew.BP_TownsfolkParentNew_C|SetIsProtected _output false)
      (Transformation|SetActorLocation _output (Math|Vector|MakeVector (.x _returnvalue) (.y _returnvalue) (+ (.z _returnvalue) 2.5e+02)) false true)
      (Pawn|Components|CharacterMovement|SetMovementMode (Variables|/Script/Engine.Character|GetCharacterMovement _output) "MOVE_Falling" 0)
      (bind _aswb_building_name (Utilities|Casting|CastToWB_BuildingName (UserInterface|GetWidget (Variables|Default|GetWidget))))
      (Default|SetUpName _aswb_building_name (Variables|Default|GetName) (Utilities|Text|ToText(String) (Utilities|String|Append (Utilities|String|ToString(Float) (Variables|Default|GetCapacity)) " out of " (Utilities|String|ToString(Float) (Variables|Default|GetMaxCapacity)) " spots left")))
      (Default|DropItem _output)
      (Utilities|Array|RemoveIndex (Variables|Default|GetTownsfolk) Index))))

(fn GetNearTownsfolk
  (return (Collision|GetOverlappingActors (Variables|Default|GetSphere) 0 :!class /Script/Engine.PrimitiveComponent)))

(fn GetOcupentbyIndex
  (params (Index :type Integer))
  (return (Utilities|Array|Get(acopy) (Variables|Default|GetTownsfolk) Index)))

(fn HasSpaceLeft
  (return (not (>= (Variables|Default|GetCapacity) (Variables|Default|GetMaxCapacity)))))

(fn CalculateScoreinBuilding
  (LocalVariables|SetLCL_LivingTownsfolk (Variables|Default|GetTownsfolk))
  (for (_array_element _array_index) (Variables|Default|GetTownsfolk)
    (bind (_usedability _abilityname _usedby _outindex) (Default|UseAbility _array_element _array_index (Variables|Default|GetTownsfolk)))
    (if _usedability
      (switch Utilities|FlowControl|Switch|SwitchonE_TownsfolkAbilities _abilityname
        (:NewEnumerator0
          (if (> (Utilities|Array|Length (LocalVariables|GetLCL_LivingTownsfolk)) 1)
            (bind _output_get (LocalVariables|SetLCL_Index (Math|Random|RandomIntegerinRange 0 (- (Utilities|Array|Length (LocalVariables|GetLCL_LivingTownsfolk)) 1)) :!label _label))
            (if (== _outindex _output_get)
              (goto _label)
              (else
                (bind _returnvalue (Utilities|Array|Add (LocalVariables|GetLCL_DeadTownsfolk) (Utilities|Array|Get(acopy) (LocalVariables|GetLCL_LivingTownsfolk) (LocalVariables|GetLCL_Index))))
                (Utilities|Array|RemoveItem (Variables|Default|GetTownsfolk) (Utilities|Array|Get(acopy) (LocalVariables|GetLCL_LivingTownsfolk) (LocalVariables|GetLCL_Index)))
                (Utilities|Array|RemoveIndex (LocalVariables|GetLCL_LivingTownsfolk) (LocalVariables|GetLCL_Index))
                (bind _asgm_werewolf_game (Utilities|Casting|CastToGM_WerewolfGame (Game|GetGameMode)))
                (Utilities|Array|Add (Variables|/Game/Player/GM_WerewolfGame.GM_WerewolfGame_C|GetUpdateSheetNotifications _asgm_werewolf_game) (Utilities|String|Append (Utilities|String|ToString(Text) (Variables|/Game/Townsfolk/BP_TownsfolkParentNew.BP_TownsfolkParentNew_C|GetName _usedby)) " has murdered " (Utilities|String|ToString(Text) (Variables|/Game/Townsfolk/BP_TownsfolkParentNew.BP_TownsfolkParentNew_C|GetName (Utilities|Array|Get(acopy) (LocalVariables|GetLCL_DeadTownsfolk) _returnvalue))) " in " (Utilities|String|ToString(Text) (Variables|Default|GetName))))))))
        (:NewEnumerator3
          (bind _returnvalue_2 (Utilities|Array|Add (LocalVariables|GetLCL_DeadTownsfolk) (Utilities|Array|Get(acopy) (LocalVariables|GetLCL_LivingTownsfolk) _outindex)))
          (Utilities|Array|RemoveItem (LocalVariables|GetLCL_LivingTownsfolk) (Utilities|Array|Get(acopy) (LocalVariables|GetLCL_LivingTownsfolk) _outindex))
          (bind _asgm_werewolf_game_2 (Utilities|Casting|CastToGM_WerewolfGame (Game|GetGameMode)))
          (Utilities|Array|Add (Variables|/Game/Player/GM_WerewolfGame.GM_WerewolfGame_C|GetUpdateSheetNotifications _asgm_werewolf_game_2) (Utilities|String|Append (Utilities|String|ToString(Text) (Variables|/Game/Townsfolk/BP_TownsfolkParentNew.BP_TownsfolkParentNew_C|GetName (Utilities|Array|Get(acopy) (LocalVariables|GetLCL_DeadTownsfolk) _returnvalue_2))) (.OutItem (Utilities|Array|Random (Utilities|Array|MakeArray " could  
stand the though  
of life without thier lover and 
went out to find them... they  
never returned" " said,  
“No werewolf will stop 
 me from finding my love!\" 
Their body was found the  
next day." (Utilities|String|Append " said,  
“No werewolf will stop 
 me from finding my love!\" 
Their body was found the  
next day." (Utilities|String|ToString(Text) (Variables|/Game/Townsfolk/BP_TownsfolkParentNew.BP_TownsfolkParentNew_C|GetName (Utilities|Array|Get(acopy) (LocalVariables|GetLCL_DeadTownsfolk) _returnvalue_2))) " died 
in the night."))))))))))
  (return (LocalVariables|GetLCL_LivingTownsfolk) (LocalVariables|GetLCL_DeadTownsfolk)))

(fn EnmptyHouse
  (if (Utilities|Array|IsNotEmpty (Variables|Default|GetTownsfolk))
    (if (== (Math|Random|RandomIntegerinRange 0 9) 0)
      (Variables|Default|SetIsLocked true)))
  (for _index (range 0 6)
    (CallFunction|RemovefromBuilding)))

(fn MouseClickon
  (Utilities|IsValid (Variables|Default|GetWidgetInfo)
    (:Is%20Not%20Valid
      (bind _returnvalue (UserInterface|CreateWidget (Variables|Default|GetInfoWidget)))
      (UserInterface|Viewport|AddtoViewport _returnvalue 0)
      (bind _output_get (Variables|Default|SetWidgetInfo _returnvalue))
      (bind _aswb_building_wbparent (Utilities|Casting|CastToWB_BuildingWBParent _output_get))
      (Default|SetUpWidget _aswb_building_wbparent (>= (.x (Transformation|GetActorLocation (Game|GetPlayerCharacter 0))) (.x (Transformation|GetActorLocation))) (Variables|Default|GetName) (Utilities|Text|ToText(String) (Utilities|String|Append (Utilities|String|ToString(Float) (Variables|Default|GetCapacity)) " out of " (Utilities|String|ToString(Float) (Variables|Default|GetMaxCapacity)) " spots left")) (Variables|Default|GetDescription) self)
      (return true))))

(fn MouseHover
  (Rendering|SetVisibility (Variables|Default|GetWidget) true false)
  (CallFunction|StartHoverCooldown)
  (return true))