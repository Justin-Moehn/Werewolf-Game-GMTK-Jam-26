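; BP_Well is a well building that townsfolk can be added to while it is usable.
; AddToBuilding passes the townsfolk to the parent only when CanUse is true, then closes the well until SetCanUseWell changes the flag.
; A separate UpdateCanUseVisuals event sets the name widget to show either remaining capacity or a safety-closure notice.
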(event Custom|SetCanUseWell
  (params (CanUse :type Boolean))
  (Variables|Default|SetCanUse CanUse))

(event Custom|UpdateCanUseVisuals
  (bind _widget (Variables|Default|GetWidget))
  (bind _returnvalue (UserInterface|GetWidget _widget))
  (if (Variables|Default|GetCanUse)
    (bind _aswb_building_name (Utilities|Casting|CastToWB_BuildingName _returnvalue))
    (Default|SetUpName _aswb_building_name (Variables|Default|GetName) (Utilities|Text|ToText(String) (Utilities|String|Append (Utilities|String|ToString(Float) (Variables|Default|GetCapacity)) " out of " (Utilities|String|ToString(Float) (Variables|Default|GetMaxCapacity)) " spots left")))
    (else
      (bind _aswb_building_name_2 (Utilities|Casting|CastToWB_BuildingName _returnvalue))
      (Default|SetUpName _aswb_building_name_2 (Variables|Default|GetName) "Blocked off for saftey reasons"))))

(event EventBeginPlay
  (|CallParentFunction) ; This node is disabled and will not be called.\nDrag off pins to build functionality.
)

(event Collision|EventActorBeginOverlap
  (params (OtherActor :type Actor%20Object%20Reference)))

(event EventTick
  (params (DeltaSeconds :type Float%20%28single-precision%29)))

(fn ConstructionScript
  (|CallParentFunction))

(fn AddtoBuilding
  (params (NewTownsfolk :type BP%20Townsfolk%20Parent%20Object%20Reference%20%28by%20ref%29))
  (if (Variables|Default|GetCanUse)
    (|CallParentFunction NewTownsfolk)
    (Variables|Default|SetCanUse false)
    (return)))