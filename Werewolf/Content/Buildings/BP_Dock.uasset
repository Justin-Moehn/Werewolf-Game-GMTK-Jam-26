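; BP_Dock is the dock building, described to the player as a place to recruit new townsfolk who arrive the next day.
; On BeginPlay it runs the parent logic, then passes its name and a recruitment title to the WB_BuildingName in its widget component.
; UpdateText switches the Description between the recruitment pitch and a wait-until-tomorrow notice based on Cooldown.
; The recruiting and cooldown logic itself is not in this Blueprint.
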(event Custom|Update%20Text
  (if (Variables|Default|GetCooldown)
    (Variables|Default|SetDescription "Wait until tomorrow to  
recuit anyone else.")
    (else
      (Variables|Default|SetDescription "This is a great place to recruit  
new townsfolk. Though they won't 
get here till tomorrow."))))

(event EventBeginPlay
  (|CallParentFunction)
  (bind _aswb_building_name (Utilities|Casting|CastToWB_BuildingName (UserInterface|GetWidget (Variables|Default|GetWidget))))
  (Default|SetUpName _aswb_building_name (Variables|Default|GetName) "Requit New Townsfolk"))

(event Collision|EventActorBeginOverlap
  (params (OtherActor :type Actor%20Object%20Reference)))

(event EventTick
  (params (DeltaSeconds :type Float%20%28single-precision%29))
  (|CallParentFunction DeltaSeconds) ; This node is disabled and will not be called.\nDrag off pins to build functionality.
)

(fn ConstructionScript
  (|CallParentFunction))